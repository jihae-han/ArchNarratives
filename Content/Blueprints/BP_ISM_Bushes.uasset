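; Bush instancer actor that rebuilds saved bush placements as instanced static meshes in its construction script.
; It loads a TransformSave from the named slot, if one exists, and assigns the saved mesh types by index to two ISM components.
; Each saved transform becomes a world-space instance on the component matching its mesh ID, with a printed warning for IDs that have no component.
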(event EventBeginPlay)

(event Collision|EventActorBeginOverlap
  (params (OtherActor :type Actor%20Object%20Reference)))

(event EventTick
  (params (DeltaSeconds :type Float%20%28single-precision%29)))

(fn ConstructionScript
  ;[1 1 1] Does save slot exist?
  (bind _returnvalue (SaveGame|DoesSaveGameExist (Variables|Default|GetSaveSlotName)))
  (bind _output_get (Variables|Default|SetSaveExists? _returnvalue))
  (if _output_get
    (bind _returnvalue_2 (SaveGame|LoadGamefromSlot (Variables|Default|GetSaveSlotName)))
    (bind _astransform_save (Utilities|Casting|CastToTransformSave _returnvalue_2))
    (LocalVariables|Setlocal_MeshIDs (Variables|/Game/Blueprints/TransformSave.TransformSave_C|GetMeshIDs _astransform_save))
    (LocalVariables|Setlocal_MeshTypes (Variables|/Game/Blueprints/TransformSave.TransformSave_C|GetMeshTypes _astransform_save))
    (bind _output_get_2 (LocalVariables|Setlocal_Transforms (Variables|/Game/Blueprints/TransformSave.TransformSave_C|GetTransforms _astransform_save)))
    (Utilities|FlowControl|Sequence
      (:then_0
        ;[1 1 1] Instance static meshes
        (for (_array_element _array_index) (LocalVariables|Getlocal_MeshTypes)
          (switch int _array_index
            (:0
              (Components|StaticMesh|SetStaticMesh (Variables|Default|GetISM_bush02) _array_element))
            (:1
              (Components|StaticMesh|SetStaticMesh (Variables|Default|GetISM_bush03) _array_element)))))
      (:then_1
        (for (_array_element_2 _array_index_2) _output_get_2
          (switch int (Utilities|Array|Get(acopy) (LocalVariables|Getlocal_MeshIDs) _array_index_2)
            (:Default
              (Development|PrintString (Utilities|String|Append "Requires \"" (Utilities|String|ToString(Integer) (.MaxValue (Math|Integer|MaxOfIntArray (LocalVariables|Getlocal_MeshIDs)))) "\" more ISMS!")))
            (:0
              (Components|InstancedStaticMesh|AddInstance (Variables|Default|GetISM_bush02) _array_element_2 true))
            (:1
              (Components|InstancedStaticMesh|AddInstance (Variables|Default|GetISM_bush03) _array_element_2 true))))))))