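; BP_Narrator procedurally generates grid-based spaces, spawns them as BP_Space actors, and can identify the PC or VR pawn's cell.
; SpliceSpaces sizes a seeded-random collider from the previous node, gathers overlapped BP_Cells, and classifies each by its neighbours into SpaceInfo, stacking transforms along Z.
; CalcNode chains exposed cell edges into an outline and traces from them, but only draws debug, returning no node.
; Data tables and NarratorSave supply layout data.
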(event Custom|SpawnSpaces
  ;[0 0 0] spawn spaces
  (Utilities|Array|Clear (Variables|Template|Getspaces))
  (for (_array_element _array_index) (Variables|Template|Getspace_Info)
    (bind _returnvalue (Game|SpawnActorfromClass "/Game/Blueprints/BP_Space.BP_Space_C" (Utilities|Array|Get(acopy) (Variables|Template|Getspace_Transforms) _array_index) "AlwaysSpawn" 0 (Variables|Template|GettileSlot) _array_element 0))
    (Utilities|Array|Add (Variables|Template|Getspaces) _returnvalue)))

(event Custom|SpliceSpaces
  ;[0 0 0] set user-defined weights
  (Aux|SetWeights)
  ;[0 0 0] clear space data
  (Aux|ClearSpaceData)
  ;[0 0 0] set Space Info and Transforms
  (for _index (range 0 (Variables|Weights|Getspace#))
    (Variables|Default|Setindex _index)
    (Utilities|FlowControl|Sequence
      (:then_0
        ;;[0 0 0] calculate Space Info
        (bind _spaceinfo (CallFunction|CalcSpaceInfo))
        (Variables|Default|SetspaceInfo _spaceinfo)
        ;;[0 0 0] Calculate connection (node) with next space
        (bind _node (CallFunction|CalcNode))
        (Variables|Default|Setnode _node))
      (:then_1
        ;;[0 0 0] Setup Space Transforms and Info
        (Utilities|Array|Add (Variables|Template|Getspace_Nodes) (Variables|Default|Getnode))
        (Utilities|Array|Add (Variables|Template|Getspace_Transforms) (Aux|GetSpaceTransform (Variables|Default|Getindex)))
        (Utilities|Array|Add (Variables|Template|Getspace_Info) (Variables|Default|GetspaceInfo))))))

(event EventBeginPlay
  ;[0 0 0] set player state
  (Aux|SetPlayerState))

(event Events|EventOnRebuildGeneratedMesh
  (params (TargetMesh :type Dynamic%20Mesh%20Object%20Reference))
  ;[0 0 0] set target mesh
  (Variables|Default|SettargetMesh TargetMesh))

(fn ConstructionScript
  (Aux|LoadData))

(fn TestDebug)

(fn GetPawnCellID
  (bind _resolution (Variables|ReadOnly|Getresolution))
  (bind _vr_pawn (Variables|Player|GetVR_Pawn))
  (bind _pc_pawn (Variables|Player|GetPC_Pawn))
  (bind _resolution_2 (Variables|ReadOnly|Getresolution))
  (bind _returnvalue (Transformation|GetActorLocation _pc_pawn))
  (bind _returnvalue_2 (Transformation|GetActorLocation _vr_pawn))
  (bind (_x _y) (Math|Vector|BreakVector _returnvalue_2))
  (bind (_x_2 _y_2) (Math|Vector|BreakVector _returnvalue))
  (switch int (Variables|Player|GetpawnState)
    (:Default
      (Development|PrintString "player not possessed" true true "(R=1.000000,G=0.000000,B=0.093744,A=1.000000)")
      (return (Utilities|Struct|MakeST_2DCoord)))
    (:0
      ;[1 1 1] player pawn get
      (return (Utilities|Struct|MakeST_2DCoord (Math|Float|Round (/ _x_2 _resolution_2)) (Math|Float|Round (/ _y_2 _resolution_2)))))
    (:1
      (return (Utilities|Struct|MakeST_2DCoord (Math|Float|Round (/ _x _resolution)) (Math|Float|Round (/ _y _resolution)))))))

(fn SpawnCells
  ;[1 1 1] spawn cells
  (for (_array_element _array_index) (Variables|Template|Getcell_Locations)
    (Game|SpawnActorfromClass "/Game/Blueprints/BP_Cell.BP_Cell_C" (Math|Transform|MakeTransform _array_element) "AlwaysSpawn" 0 (Variables|ReadOnly|Getresolution) (Utilities|Array|Get(acopy) (Variables|Template|Getcell_Pts) _array_index) 0)))

(fn LoadNarrator
  (bind _returnvalue (SaveGame|DoesSaveGameExist (Variables|Template|GetsaveSlot)))
  (if _returnvalue
    (bind _returnvalue_2 (SaveGame|LoadGamefromSlot (Variables|Template|GetsaveSlot)))
    (bind _asnarrator_save (Utilities|Casting|CastToNarratorSave _returnvalue_2)
      (:then
        (Variables|Template|Setcell_Locations (Variables|/Game/Blueprints/NarratorSave.NarratorSave_C|Getcell_locations _asnarrator_save))
        (Variables|Template|Setcell_Pts (Variables|/Game/Blueprints/NarratorSave.NarratorSave_C|Getcell_enums _asnarrator_save))
        (Variables|Template|Setcell_IDs (Variables|/Game/Blueprints/NarratorSave.NarratorSave_C|Getcell_ID _asnarrator_save))
        (Variables|Template|Setspace_Info (Variables|/Game/Blueprints/NarratorSave.NarratorSave_C|Getspace_info _asnarrator_save))
        (Variables|Template|Setspace_Transforms (Variables|/Game/Blueprints/NarratorSave.NarratorSave_C|Getspace_transforms _asnarrator_save)))
      (:CastFailed
        (Development|PrintString "Cast to Narrator save failed!" true true "(R=1.000000,G=0.000000,B=0.524104,A=1.000000)")))))

(fn SetPlayerState
  (bind _returnvalue (Game|Player|GetPlayerPawn 0))
  (Utilities|FlowControl|Sequence
    (:then_0
      (bind _asbp_top_down_character (Utilities|Casting|CastToBP_TopDownCharacter _returnvalue)
        (:then
          (Variables|Player|SetPC_Pawn _asbp_top_down_character)
          (Variables|Player|SetpawnState 0))
        (:CastFailed
          (bind _asvrpawn (Utilities|Casting|CastToVRPawn _returnvalue))
          (Variables|Player|SetVR_Pawn _asvrpawn)
          (Variables|Player|SetpawnState 1))))
    (:then_1
      (return (Variables|Player|GetpawnState)))))

(fn LoadData
  (Utilities|FlowControl|Sequence
    (:then_0
      (bind _returnvalue (SaveGame|DoesSaveGameExist (Variables|Template|GetsaveSlot)))
      (Variables|Default|SetbSave _returnvalue))
    (:then_1
      (bind _returnvalue_2 (Utilities|GetDataTableRow (Variables|ReadOnly|GetboundsDataTable) (Variables|Template|GetboundsSlot))
        (:then
          (Variables|Template|SetPE_Bounds (.boundaryPts (Utilities|Struct|BreakST_Boundary _returnvalue_2))))
        (:RowNotFound
          (Development|PrintString "Hello"))))
    (:then_2
      (bind _returnvalue_3 (Utilities|GetDataTableRow (Variables|ReadOnly|GettileDataTable) (Variables|Template|GettileSlot))
        (:then
          (Variables|Template|SettileMap (.TileMap (Utilities|Struct|BreakST_TileMap _returnvalue_3))))))))

(fn SetWeights
  ;[1 1 1] set weighted max dimension
  (Variables|Weights|SetwMaxDim (Math|Float|Truncate (* (Variables|Weights|GetsizeFactor) (Variables|Weights|GetmaxDim)))))

(fn ClearSpaceData
  (Utilities|Array|Clear (Variables|Template|Getspaces))
  (Utilities|Array|Clear (Variables|Template|Getspace_Nodes))
  (Utilities|Array|Clear (Variables|Template|Getspace_Info))
  (Utilities|Array|Clear (Variables|Template|Getspace_Transforms)))

(fn GetSpaceTransform
  (params (# :type Integer))
  (bind _returnvalue (Transformation|GetActorLocation))
  (return (Math|Transform|MakeTransform (Math|Vector|MakeVector (.x _returnvalue) (.y _returnvalue) (* # (Variables|Weights|GetspaceZ))))))

(fn CalcSpaceInfo
  (bind _resolution (Variables|ReadOnly|Getresolution))
  (bind _returnvalue (* _resolution -0.2))
  (Math|Integer|CompareInt (Variables|Default|Getindex)
    (:>
      _)
    (:==
      ;[1 1 1] Make node for Space# == 0
      (Variables|Default|Setnode (Utilities|Struct|MakeST_Node "(X=0.000000,Y=200.000000)" "(X=0.000000,Y=100.000000)"))))
  ;[1 1 1] For Space# > 0
  (Utilities|FlowControl|Sequence
    (:then_0
      ;[0 0 0] length of node segment
      (LocalVariables|Setlength (Math|Vector|Distance2D(Vector) (.start (Variables|Default|Getnode)) (.end (Variables|Default|Getnode))))
      ;[0 0 0] get direction that points <INTO> the space being generated
      (LocalVariables|Setlength_Dir (Math|Vector2D|Normalize2D (- (.end (Variables|Default|Getnode)) (.start (Variables|Default|Getnode)))))
      (LocalVariables|Setdepth_Dir (Class|KismetMathLibrary|GetRotated2D (Math|Vector2D|Normalize2D (- (.end (Variables|Default|Getnode)) (.start (Variables|Default|Getnode)))) 9e+01))
      ;[0 0 0] get random length and depth (NOTE: length is always aligned with previous node)
      (bind _output_get (LocalVariables|Setlength_Ext (Math|Random|RandomIntegerinRangefromStream 0 (Variables|Weights|GetwMaxDim) (Variables|Template|GetrandStream))))
      (LocalVariables|Setlength (+ (LocalVariables|Getlength) (* _output_get (Variables|ReadOnly|Getresolution))))
      (LocalVariables|Setdepth (* (Math|Random|RandomIntegerinRangefromStream (Variables|ReadOnly|GetminDim) (Variables|Weights|GetwMaxDim) (Variables|Template|GetrandStream)) (Variables|ReadOnly|Getresolution)))
      ;[0 0 0] Set collider extents
      (Components|Box|SetBoxExtent (Variables|Default|GetCollider) (* (Math|Vector|MakeVector (.x (+ (Class|KismetMathLibrary|GetAbs2D (* (LocalVariables|Getdepth_Dir) (Math|Vector2D|MakeVector2D (LocalVariables|Getdepth) (LocalVariables|Getdepth)))) (Class|KismetMathLibrary|GetAbs2D (* (LocalVariables|Getlength_Dir) (Math|Vector2D|MakeVector2D (LocalVariables|Getlength) (LocalVariables|Getlength)))) (Math|Vector2D|MakeVector2D _returnvalue _returnvalue))) (.y (+ (Class|KismetMathLibrary|GetAbs2D (* (LocalVariables|Getdepth_Dir) (Math|Vector2D|MakeVector2D (LocalVariables|Getdepth) (LocalVariables|Getdepth)))) (Class|KismetMathLibrary|GetAbs2D (* (LocalVariables|Getlength_Dir) (Math|Vector2D|MakeVector2D (LocalVariables|Getlength) (LocalVariables|Getlength)))) (Math|Vector2D|MakeVector2D _returnvalue _returnvalue))) 3e+02) 0.5) true))
    (:then_1
      ;[0 0 0] get random space offset (along axis with node)
      (LocalVariables|Setoffset (* (Math|Random|RandomIntegerinRangefromStream 0 (Variables|Weights|GetwMaxDim) (Variables|Template|GetrandStream)) (Variables|ReadOnly|Getresolution) -1.0))
      ;[0 0 0] calculate collider origin
      (Transformation|SetWorldLocation (Variables|Default|GetCollider) (+ (* (Math|Vector|MakeVector (.x (+ (* (LocalVariables|Getdepth_Dir) (Math|Vector2D|MakeVector2D (LocalVariables|Getdepth) (LocalVariables|Getdepth))) (* (LocalVariables|Getlength_Dir) (Math|Vector2D|MakeVector2D (LocalVariables|Getlength) (LocalVariables|Getlength))) (* (LocalVariables|Getlength_Dir) (Math|Vector2D|MakeVector2D (LocalVariables|Getoffset) (LocalVariables|Getoffset))))) (.y (+ (* (LocalVariables|Getdepth_Dir) (Math|Vector2D|MakeVector2D (LocalVariables|Getdepth) (LocalVariables|Getdepth))) (* (LocalVariables|Getlength_Dir) (Math|Vector2D|MakeVector2D (LocalVariables|Getlength) (LocalVariables|Getlength))) (* (LocalVariables|Getlength_Dir) (Math|Vector2D|MakeVector2D (LocalVariables|Getoffset) (LocalVariables|Getoffset))))) 3e+02) 0.5) (.start (Variables|Default|Getnode))) false true)
      ;[0 0 0] set cell ids
      (for _array_element (Collision|GetOverlappingActors (Variables|Default|GetCollider) "/Game/Blueprints/BP_Cell.BP_Cell_C" :!class /Script/Engine.PrimitiveComponent)
        (bind _asbp_cell (Utilities|Casting|CastToBP_Cell _array_element))
        (Utilities|Array|Add (LocalVariables|Getlocal_ids) (Variables|/Game/Blueprints/BP_Cell.BP_Cell_C|GetID _asbp_cell))))
    (:then_2
      ;[0 0 0] setup local enums and keys
      (Utilities|Map|Clear (Variables|Default|Getsegments))
      (for _array_element_2 (LocalVariables|Getlocal_ids)
        (bind _enum (CallFunction|GetCellInfo _array_element_2 (LocalVariables|Getlocal_ids))) ; E & Segments
        (bind _output_get_2 (LocalVariables|Setenum _enum))
        (Utilities|Array|AddUnique (LocalVariables|Getlocal_es) _output_get_2)
        (Utilities|Array|Add (LocalVariables|Getlocal_keys) (Utilities|Array|FindItem (LocalVariables|Getlocal_es) (LocalVariables|Getenum))))
      ;[0 0 0] make space info
      (return (Utilities|Struct|MakeST_SpaceInfo (LocalVariables|Getlocal_es) (LocalVariables|Getlocal_keys) (LocalVariables|Getlocal_ids) (Variables|Default|Getindex))))))

(fn GetCellInfo
  (params (id :type ST%202D%20Coord%20Structure%20%28by%20ref%29) (search :type Array%20of%20ST%202D%20Coord%20Structures))
  (bind (_x _y) (Utilities|Struct|BreakST_2DCoord id))
  (bind (_x_2 _y_2) (Utilities|Struct|BreakST_2DCoord id))
  (bind (_x_3 _y_3) (Utilities|Struct|BreakST_2DCoord id))
  (bind _local_segments (LocalVariables|Getlocal_segments))
  (bind _resolution (Variables|ReadOnly|Getresolution))
  (bind _resolution_2 (Variables|ReadOnly|Getresolution))
  (bind _local_segments_2 (LocalVariables|Getlocal_segments))
  (bind _returnvalue (+ _x_2 1))
  (bind _returnvalue_2 (+ _y_2 1))
  (bind _returnvalue_3 (- _y_2 1))
  (bind _returnvalue_4 (- _x_2 1))
  (bind _returnvalue_5 (* _resolution _y))
  (bind _returnvalue_6 (* _x _resolution))
  (bind _returnvalue_7 (* _resolution_2 0.5))
  (bind _returnvalue_8 (* _resolution_2 -0.5))
  (bind _returnvalue_9 (+ _returnvalue_6 _returnvalue_7))
  (bind _returnvalue_10 (+ _returnvalue_6 _returnvalue_8))
  (bind _returnvalue_11 (+ _returnvalue_5 _returnvalue_7))
  (bind _returnvalue_12 (+ _returnvalue_5 _returnvalue_8))
  (Utilities|FlowControl|Sequence
    (:then_0
      ;[0 0 0] check cell adjacencies
      (Utilities|FlowControl|Sequence
        (:then_0
          (bind _output_get (LocalVariables|Setlocal_coord (Utilities|Struct|MakeST_2DCoord _returnvalue _returnvalue_2))) ; (+1,+1)
          (if (Utilities|Array|ContainsItem search _output_get)
            (LocalVariables|Setstr (Utilities|String|Append (LocalVariables|Getstr) "0"))))
        (:then_1
          (bind _output_get_2 (LocalVariables|Setlocal_coord (Utilities|Struct|MakeST_2DCoord _returnvalue _y_3))) ; (+1,0)
          (if (Utilities|Array|ContainsItem search _output_get_2)
            (LocalVariables|Setstr (Utilities|String|Append (LocalVariables|Getstr) "1"))
            (else
              ;[0 0 0] Find Bounds (edges)
              (Utilities|Map|Add _local_segments_2 (Math|Vector2D|MakeVector2D _returnvalue_9 _returnvalue_12) (Math|Vector2D|MakeVector2D _returnvalue_9 _returnvalue_11)) ; 1 (+1,0)
            )))
        (:then_2
          (bind _output_get_3 (LocalVariables|Setlocal_coord (Utilities|Struct|MakeST_2DCoord _returnvalue _returnvalue_3))) ; (+1,-1)
          (if (Utilities|Array|ContainsItem search _output_get_3)
            (LocalVariables|Setstr (Utilities|String|Append (LocalVariables|Getstr) "2"))))
        (:then_3
          (bind _output_get_4 (LocalVariables|Setlocal_coord (Utilities|Struct|MakeST_2DCoord _x_3 _returnvalue_3))) ; (0,-1)
          (if (Utilities|Array|ContainsItem search _output_get_4)
            (LocalVariables|Setstr (Utilities|String|Append (LocalVariables|Getstr) "3"))
            (else
              (Utilities|Map|Add _local_segments_2 (Math|Vector2D|MakeVector2D _returnvalue_10 _returnvalue_12) (Math|Vector2D|MakeVector2D _returnvalue_9 _returnvalue_12)) ; 3 (0,-1)
            )))
        (:then_4
          (bind _output_get_5 (LocalVariables|Setlocal_coord (Utilities|Struct|MakeST_2DCoord _returnvalue_4 _returnvalue_3))) ; (-1,-1)
          (if (Utilities|Array|ContainsItem search _output_get_5)
            (LocalVariables|Setstr (Utilities|String|Append (LocalVariables|Getstr) "4"))))
        (:then_5
          (bind _output_get_6 (LocalVariables|Setlocal_coord (Utilities|Struct|MakeST_2DCoord _returnvalue_4 _y_3))) ; (-1,0)
          (if (Utilities|Array|ContainsItem search _output_get_6)
            (LocalVariables|Setstr (Utilities|String|Append (LocalVariables|Getstr) "5"))
            (else
              (Utilities|Map|Add _local_segments_2 (Math|Vector2D|MakeVector2D _returnvalue_10 _returnvalue_11) (Math|Vector2D|MakeVector2D _returnvalue_10 _returnvalue_12)) ; 5 (-1,0)
            )))
        (:then_6
          (bind _output_get_7 (LocalVariables|Setlocal_coord (Utilities|Struct|MakeST_2DCoord _returnvalue_4 _returnvalue_2))) ; (-1,+1)
          (if (Utilities|Array|ContainsItem search _output_get_7)
            (LocalVariables|Setstr (Utilities|String|Append (LocalVariables|Getstr) "6"))))
        (:then_7
          (bind _output_get_8 (LocalVariables|Setlocal_coord (Utilities|Struct|MakeST_2DCoord _x_3 _returnvalue_2))) ; (0,+1)
          (if (Utilities|Array|ContainsItem search _output_get_8)
            (LocalVariables|Setstr (Utilities|String|Append (LocalVariables|Getstr) "7"))
            (else
              (Utilities|Map|Add _local_segments_2 (Math|Vector2D|MakeVector2D _returnvalue_9 _returnvalue_11) (Math|Vector2D|MakeVector2D _returnvalue_10 _returnvalue_11)) ; 7 (0,+1)
            )))
        (:then_8
          ;;[0 0 0] add local segments to global segment variable
          (Utilities|FlowControl|Sequence
            (:then_0
              ;;[0 0 0] figure out corner point
              (bind _values (Utilities|Map|Values (LocalVariables|Getlocal_segments)))
              (Math|Integer|CompareInt (Utilities|Array|Length _values) 1
                (:>
                  (for _array_element _values
                    (if (.ReturnValue (Utilities|Map|Find (LocalVariables|Getlocal_segments) _array_element))
                      (Variables|Default|SetboundsPt _array_element))))))
            (:then_1
              (bind _keys (Utilities|Map|Keys _local_segments))
              (for _array_element_2 _keys
                (if (.ReturnValue (Utilities|Map|Find _local_segments _array_element_2))
                  (Utilities|Map|Add (Variables|Default|Getsegments) _array_element_2 (.Value (Utilities|Map|Find _local_segments _array_element_2)))
                  (else
                    (Development|PrintString "local_segment not found")))))))))
    (:then_1
      ;[0 0 0] Set enums
      (switch string (LocalVariables|Getstr)
        (:Default
          (return "NewEnumerator2"))
        (:01237
          (return "NewEnumerator6"))
        (:12345
          (return "NewEnumerator3"))
        (:01567
          (return "NewEnumerator4"))
        (:34567
          (return "NewEnumerator5"))
        (:345
          (return "NewEnumerator7"))
        (:567
          (return "NewEnumerator8"))
        (:123
          (return "NewEnumerator9"))
        (:017
          (return "NewEnumerator10"))
        (:3
          (return "NewEnumerator13"))
        (:7
          (return "NewEnumerator14"))
        (:5
          (return "NewEnumerator15"))
        (:1
          (return "NewEnumerator16"))
        (:01234567
          (return "NewEnumerator1"))))))

(fn CalcNode
  (bind _local_bounds (LocalVariables|Getlocal_bounds))
  (bind _local_bounds_2 (LocalVariables|Getlocal_bounds))
  (bind _tracelim (Variables|ReadOnly|GettraceLim))
  (bind _resolution (Variables|ReadOnly|Getresolution))
  (bind _returnvalue (Utilities|Array|LastIndex _local_bounds))
  (Utilities|FlowControl|Sequence
    (:then_0
      ;[0 0 0] Order vectors in bounds
      (bind _keys (Utilities|Map|Keys (Variables|Default|Getsegments)))
      (bind _output_get (LocalVariables|Setlocal_key (Variables|Default|GetboundsPt)))
      (Utilities|Array|Add (LocalVariables|Getlocal_bounds) _output_get)
      (for _index (range 0 (Utilities|Array|LastIndex _keys))
        (if (.ReturnValue (Utilities|Map|Find (Variables|Default|Getsegments) (LocalVariables|Getlocal_key)))
          (bind _output_get_2 (LocalVariables|Setlocal_key (.Value (Utilities|Map|Find (Variables|Default|Getsegments) (LocalVariables|Getlocal_key)))))
          (Utilities|Array|Add (LocalVariables|Getlocal_bounds) _output_get_2)
          (else
            (Development|PrintString "segment not found"))))
      ;[0 0 0] debuggin only
      (for (_array_element _array_index) _local_bounds
        (Math|Integer|CompareInt _array_index _returnvalue
          (:<
            (Rendering|Debug|DrawDebugLine (Math|Conversions|ToVector(Vector2D) _array_element) (Math|Conversions|ToVector(Vector2D) (Utilities|Array|Get(acopy) (LocalVariables|Getlocal_bounds) (+ _array_index 1))) "(R=1.000000,G=0.000000,B=0.874681,A=1.000000)" 5.0 1.0)
            (Rendering|Debug|DrawDebugString (Math|Conversions|ToVector(Vector2D) _array_element) (Utilities|String|ToString(Integer) _array_index) 0 "(R=0.000000,G=0.000000,B=0.000000,A=1.000000)" 5.0))))
      (Development|PrintString (Utilities|String|ToString(Integer) _returnvalue) true true "(R=0.000000,G=0.660000,B=1.000000,A=1.000000)" 5.0))
    (:then_1
      (bind _output_get_3 (LocalVariables|Setlocal_count (- (Utilities|Array|LastIndex (LocalVariables|Getlocal_bounds)) 1)))
      (for _index_2 (range 0 _output_get_3)
        (LocalVariables|Setlocal_curr (Utilities|Array|Get(acopy) _local_bounds_2 _index_2))
        (LocalVariables|Setlocal_next (Utilities|Array|Get(acopy) _local_bounds_2 (+ _index_2 1)))
        (LocalVariables|Setlocal_dir (Math|Vector2D|Normalize2D (- (LocalVariables|Getlocal_next) (LocalVariables|Getlocal_curr))))
        (bind _output_get_4 (LocalVariables|Setlocal_midpt (* (Math|Conversions|ToVector(Vector2D) (+ (Utilities|Array|Get(acopy) _local_bounds_2 _index_2) (Utilities|Array|Get(acopy) _local_bounds_2 (+ _index_2 1))) 1.0) 0.5)))
        (bind _outhits (Class|KismetSystemLibrary|LineTraceMultiforObjects _output_get_4 (+ (LocalVariables|Getlocal_midpt) (* (Class|KismetMathLibrary|GetRotated2D (Math|Vector2D|Normalize2D (- (LocalVariables|Getlocal_next) (LocalVariables|Getlocal_curr))) 9e+01) (Math|Vector2D|MakeVector2D _tracelim _tracelim))) (Variables|ReadOnly|GetcellCollisionType) false 0 "None" true))
        (for _array_element_2 _outhits
          (Rendering|Debug|DrawDebugArrow (.ImpactPoint (Collision|BreakHitResult _array_element_2)) (+ (.ImpactPoint (Collision|BreakHitResult _array_element_2)) (* (Class|KismetMathLibrary|GetRotated2D (LocalVariables|Getlocal_dir) 9e+01) (Math|Vector|MakeVector _resolution _resolution 0.0))) 4.0 "(R=0.000000,G=0.000000,B=0.000000,A=1.000000)" 5.0 1.0))))))