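; Modular level space that builds itself from SpaceInfo and a tile data table, and can rise, lower and fade.
; Construction creates instanced meshes per cell type, places door instances at node midpoints and fits a box collider to the last node, leading to the next space.
; Rise timeline moves the actor by SpaceZ, while Fade timeline drives a "Fade" parameter on dynamic materials collected during construction.
; An event hides doors and disables collider overlaps.
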(event Custom|FadeIn
  ;[0 0 0] Fade In
  (bind _incr (Timeline|Fade Play)
    (:Update
      (bind _output_get (Variables|Default|SetfadeValue _incr))
      (for _array_element (Variables|Default|GetdynMaterials)
        (Rendering|Material|SetScalarParameterValue _array_element "Fade" _output_get :!class /Script/Engine.MaterialInstanceDynamic)))))

(event Custom|hideDoor
  (Development|SetHiddeninGame (Variables|Default|GetdoorISM) true true)
  (Variables|/Script/Engine.PrimitiveComponent|SetbGenerateOverlapEvents (Variables|Default|Getcollider) false))

(event Custom|FadeOut
  ;[0 0 0] Fade In
  (bind _incr (Timeline|Fade ReverseFromEnd)
    (:Update
      (bind _output_get (Variables|Default|SetfadeValue _incr))
      (for _array_element (Variables|Default|GetdynMaterials)
        (Rendering|Material|SetScalarParameterValue _array_element "Fade" _output_get :!class /Script/Engine.MaterialInstanceDynamic)))))

(event EventUp
  (bind _returnvalue (Transformation|GetActorLocation))
  ;[0 0 0] Control Vertical Movement of Space
  (Utilities|FlowControl|Sequence
    (:then_0
      (if (Audio|Components|Audio|IsPlaying (Variables|Default|GetRise))
        (bind _incr (Timeline|Rise Play)
          (:Update
            (Transformation|SetActorLocation (+ (Variables|Default|Getlocation) (Math|Vector|MakeVector 0.0 0.0 (* _incr (Variables|ReadOnly|GetspaceZ)))) false true))
          (:Finished
            (Variables|Default|Setlocation (Transformation|GetActorLocation))))
        (else
          (Variables|Default|Setlocation (Transformation|GetActorLocation))
          (Timeline|Rise PlayFromStart))))
    (:then_1
      (Math|Float|CompareFloat (.z _returnvalue) (Utilities|Operators|Subtract (.z _returnvalue) (Variables|ReadOnly|GetspaceZ) 1e+01)
        (:>
          (Math|Float|CompareFloat (Variables|Default|GetfadeValue) 0.1
            (:<
              (CallFunction|Fadein))))))))

(event EventDown
  ;[0 0 0] Control Vertical Movement of Space
  (Utilities|FlowControl|Sequence
    (:then_0
      (if (Audio|Components|Audio|IsPlaying (Variables|Default|GetRise))
        (bind _incr (Timeline|Rise Reverse)
          (:Update
            (Transformation|SetActorLocation (+ (Variables|Default|Getlocation) (Math|Vector|MakeVector 0.0 0.0 (* _incr (Variables|ReadOnly|GetspaceZ)))) false true))
          (:Finished
            (Variables|Default|Setlocation (Transformation|GetActorLocation))))
        (else
          (Variables|Default|Setlocation (- (Transformation|GetActorLocation) (Math|Vector|MakeVector 0.0 0.0 (Variables|ReadOnly|GetspaceZ))))
          (Timeline|Rise ReverseFromEnd))))
    (:then_1
      (Math|Float|CompareFloat (.z (Transformation|GetActorLocation)) 1e+01
        (:<
          (Math|Float|CompareFloat (Variables|Default|GetfadeValue) 0.9
            (:>
              (CallFunction|FadeOut))))))))

(fn ConstructionScript
  (bind _spaceinfo (Variables|Default|GetspaceInfo))
  (Utilities|FlowControl|Sequence
    (:then_0
      ;[0 0 0] load tile data table
      (bind _returnvalue (Utilities|GetDataTableRow (Variables|ReadOnly|GettileDataTable) (Variables|Default|GettileSlot))
        (:then
          (Variables|ReadOnly|SettileMap (.TileMap (Utilities|Struct|BreakST_TileMap _returnvalue)))
          (Variables|ReadOnly|Setresolution (.Spacing (Utilities|Struct|BreakST_TileMap _returnvalue))))))
    (:then_1
      ;[0 0 0] Break up variables from Space Info
      (Variables|Default|Setcell_Es (.cell_e _spaceinfo))
      (Variables|Default|Setcell_Keys (.cell_keys _spaceinfo))
      (Variables|Default|Setcell_IDs (.cell_coords _spaceinfo))
      (Variables|Default|Setnodes (.nodes _spaceinfo))
      (Variables|Default|Set# (.none _spaceinfo)))
    (:then_2
      ;[0 0 0] Add door portal instances
      (Components|StaticMesh|SetStaticMesh (Variables|Default|GetdoorISM) (.Value (Utilities|Map|Find (Variables|ReadOnly|GettileMap) "NewEnumerator22")))
      (for _array_element (Variables|Default|Getnodes)
        (Math|Float|CompareFloat (.x (Class|KismetMathLibrary|GetAbs2D (- (.End (Utilities|Struct|BreakST_Node _array_element)) (.Start (Utilities|Struct|BreakST_Node _array_element))))) (.y (Class|KismetMathLibrary|GetAbs2D (- (.End (Utilities|Struct|BreakST_Node _array_element)) (.Start (Utilities|Struct|BreakST_Node _array_element)))))
          (:>
            (LocalVariables|SetdoorRotation "0,90.000000, 0"))
          (:<
            (LocalVariables|SetdoorRotation "0, 0, 0")))
        (Components|InstancedStaticMesh|AddInstance (Variables|Default|GetdoorISM) (Math|Transform|MakeTransform (Math|Conversions|ToVector(Vector2D) (* (+ (.Start (Utilities|Struct|BreakST_Node _array_element)) (.End (Utilities|Struct|BreakST_Node _array_element))) "(X=0.500000,Y=0.500000)") (.z (Transformation|GetActorLocation))) (LocalVariables|GetdoorRotation) "1.000000,1.000000,1.000000") true)
        ;;[0 0 0] Set Dynamic Masterials
        (CallFunction|SetDynMaterials (Variables|Default|GetdoorISM))))
    (:then_3
      ;[0 0 0] add node collider to next space
      (Transformation|SetRelativeTransform (Variables|Default|Getcollider) (Math|Transform|MakeTransform (* (Math|Conversions|ToVector(Vector2D) (+ (.Start (Utilities|Struct|BreakST_Node (Utilities|Array|Get(acopy) (Variables|Default|Getnodes) (Utilities|Array|LastIndex (Variables|Default|Getnodes))))) (.End (Utilities|Struct|BreakST_Node (Utilities|Array|Get(acopy) (Variables|Default|Getnodes) (Utilities|Array|LastIndex (Variables|Default|Getnodes)))))) (Variables|ReadOnly|GetnodeHeight)) 0.5) (Math|Rotator|CombineRotators (Math|Rotator|FindLookatRotation (Math|Conversions|ToVector(Vector2D) (.End (Utilities|Struct|BreakST_Node (Utilities|Array|Get(acopy) (Variables|Default|Getnodes) (Utilities|Array|LastIndex (Variables|Default|Getnodes)))))) (Math|Conversions|ToVector(Vector2D) (.Start (Utilities|Struct|BreakST_Node (Utilities|Array|Get(acopy) (Variables|Default|Getnodes) (Utilities|Array|LastIndex (Variables|Default|Getnodes))))))) "0,90.000000, 0")) false true)
      (Components|Box|SetBoxExtent (Variables|Default|Getcollider) (Math|Vector|MakeVector 1e+01 (* (Math|Vector|Distance2D(Vector) (.Start (Utilities|Struct|BreakST_Node (Utilities|Array|Get(acopy) (Variables|Default|Getnodes) (Utilities|Array|LastIndex (Variables|Default|Getnodes))))) (.End (Utilities|Struct|BreakST_Node (Utilities|Array|Get(acopy) (Variables|Default|Getnodes) (Utilities|Array|LastIndex (Variables|Default|Getnodes)))))) 0.5) (* (Variables|ReadOnly|GetnodeHeight) 0.5)) true))
    (:then_4
      ;[0 0 0] add instanced meshes
      (for (_array_element_2 _array_index) (Variables|Default|Getcell_Es)
        (bind _returnvalue_2 (AddComponent|AddInstancedStaticMeshComponent false))
        (if (.ReturnValue (Utilities|Map|Find (Variables|ReadOnly|GettileMap) _array_element_2))
          (Components|StaticMesh|SetStaticMesh _returnvalue_2 (.Value (Utilities|Map|Find (Variables|ReadOnly|GettileMap) _array_element_2)))
          ;;[0 0 0] create Dynamic Materials
          (CallFunction|SetDynMaterials _returnvalue_2)
          (for (_array_element_3 _array_index_2) (Variables|Default|Getcell_Keys)
            (if (== _array_index _array_element_3)
              (Components|InstancedStaticMesh|AddInstance _returnvalue_2 (Math|Transform|MakeTransform (Math|Vector|MakeVector (* (.x (Utilities|Array|Get(acopy) (Variables|Default|Getcell_IDs) _array_index_2)) (Variables|ReadOnly|Getresolution)) (* (.y (Utilities|Array|Get(acopy) (Variables|Default|Getcell_IDs) _array_index_2)) (Variables|ReadOnly|Getresolution)) (.z (Transformation|GetActorLocation)))) true))))))
    (:then_5
      ;;[1 1 1] hide meshes > 2
      (Math|Integer|CompareInt (Variables|Default|Get#) 2
        (:>
          (for _array_element_4 (Variables|Default|GetdynMaterials)
            (Rendering|Material|SetScalarParameterValue _array_element_4 "Fade" 0.0 :!class /Script/Engine.MaterialInstanceDynamic)))))))

(fn GetColliderForward
  (return (Math|Vector|GetForwardVector (Variables|Default|Getcollider))))

(fn SetDynMaterials
  (params (meshComponent :type Mesh%20Component%20Object%20Reference%20%28by%20ref%29))
  (for (_array_element _array_index) (Rendering|Material|GetMaterials meshComponent)
    (bind _returnvalue (Rendering|Material|CreateDynamicMaterialInstance meshComponent _array_index _array_element "None" :!class /Script/Engine.PrimitiveComponent))
    (Rendering|Material|SetMaterial meshComponent _array_index _returnvalue)
    (Utilities|Array|Add (Variables|Default|GetdynMaterials) _returnvalue)))