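; BP_Cell is a grid cell actor that identifies its 2D coordinate from its world position.
; Its construction script sizes a box collider to the Resolution footprint with fixed height and puts it on a custom object channel.
; It then divides the actor location by Resolution and rounds it to set IDX, IDY and an ST2DCoord ID, and GetID returns the X and Y indices.
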(event EventBeginPlay)

(event Collision|EventActorBeginOverlap
  (params (OtherActor :type Actor%20Object%20Reference)))

(event EventTick
  (params (DeltaSeconds :type Float%20%28single-precision%29)))

(fn ConstructionScript
  (bind _returnvalue (Transformation|GetActorLocation))
  (bind _resolution (Variables|Default|Getresolution))
  (bind _resolution_2 (Variables|Default|Getresolution))
  (bind (_x _y) (Math|Vector|BreakVector _returnvalue))
  (bind _returnvalue_2 (* _resolution_2 0.5))
  ;[1 1 1] Set box collider extents
  (Collision|SetCollisionObjectType (Variables|Default|GetCollider) "ECC_GameTraceChannel2")
  (Components|Box|SetBoxExtent (Variables|Default|GetCollider) (Math|Vector|MakeVector _returnvalue_2 _returnvalue_2 1.5e+02) true)
  ;[1 1 1] set coord_ID
  (bind _output_get (Variables|Default|SetID_X (Math|Float|Round (/ _x _resolution))))
  (bind _output_get_2 (Variables|Default|SetID_Y (Math|Float|Round (/ _y _resolution))))
  (Variables|Default|SetID (Utilities|Struct|MakeST_2DCoord _output_get _output_get_2)))

(fn GetID
  (return (Variables|Default|GetID_X) (Variables|Default|GetID_Y)))